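; BP_Homework is a clickable prop actor whose Type variable selects one of four reactions when EV_Click fires.
; It either adds a particle system component or toggles the Cube mesh's relative location, rotation, or "Power" material parameter.
; Each toggle uses a FlipFlop to play or reverse its own Timeline, which drives a Lerp.
; The construction script assigns the meshes for Cube and Cube1 from variables.
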(event Custom|EV_Click
  (switch int (Variables|Default|GetType)
    (:0
      (AddComponent|AddParticleSystemComponent false))
    (:1
      (Utilities|FlowControl|FlipFlop
        (:A
          (bind _newtrack_0 (Timeline|Timeline Play)
            (:Update
              (Transformation|SetRelativeLocation (Variables|Default|GetCube) (Math|Vector|Lerp(Vector) "0, 0, 0" (Variables|Default|GetAfter%20Position) _newtrack_0) false false))))
        (:B
          (Timeline|Timeline Reverse))))
    (:2
      (Utilities|FlowControl|FlipFlop
        (:A
          (bind _newtrack_0_2 (Timeline|Timeline_0 Play)
            (:Update
              (Transformation|SetRelativeRotation (Variables|Default|GetCube) (Math|Rotator|Lerp(Rotator) "0, 0, 0" (Variables|Default|GetAfter%20Rotation) _newtrack_0_2) false false))))
        (:B
          (Timeline|Timeline_0 Reverse))))
    (:3
      (Utilities|FlowControl|FlipFlop
        (:A
          (bind _newtrack_0_3 (Timeline|Timeline_1 Play)
            (:Update
              (Rendering|Material|SetScalarParameterValueonMaterials (Variables|Default|GetCube) "Power" (Math|Float|Lerp 0.0 5e+01 _newtrack_0_3)))))
        (:B
          (Timeline|Timeline_1 Reverse))))))

(fn ConstructionScript
  (Components|StaticMesh|SetStaticMesh (Variables|Default|GetCube) (Variables|Default|GetSM%20Mesh%2001))
  (Components|StaticMesh|SetStaticMesh (Variables|Default|GetCube1) (Variables|Default|GetSM%20Mesh%2002)))