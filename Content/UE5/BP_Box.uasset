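; BP_Box is a test actor whose Cube component steps up in height each time the player presses the 2 key.
; On BeginPlay it enables input from player controller 0.
; Each press increments a counter that wraps to zero after ten, and the cube's relative Z is set to that count times a fixed spacing.
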(event EventBeginPlay
  (Input|EnableInput (Game|GetPlayerController 0)))

(event Input|KeyboardEvents|2
  (params (Key :type Key%20Structure :default "None"))
  (:Pressed
    (Variables|Default|SetNum (+ (Variables|Default|GetNum) 1))
    (if (> (Variables|Default|GetNum) 10)
      (Variables|Default|SetNum 0))
    (Transformation|SetRelativeLocation (Variables|Default|GetCube) (Math|Vector|MakeVector 0.0 0.0 (Math|Conversions|ToFloat(Integer) (* (Variables|Default|GetNum) 100))) false false)))

(fn ConstructionScript)