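; Elevator actor that moves its inside mesh up or down, alternating each time its trigger box is overlapped.
; An overlap casts player pawn 0, rather than the overlapping actor, to BP_ThirdPersonCharacter and calls its EvCam event.
; A FlipFlop then plays or reverses a timeline that lerps the mesh's relative Z between zero and a target height.
; The construction script sets the mesh's initial relative Z.
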(event OnComponentBeginOverlap(Box)
  (params (OverlappedComponent :type Primitive%20Component%20Object%20Reference) (OtherActor :type Actor%20Object%20Reference) (OtherComp :type Primitive%20Component%20Object%20Reference) (OtherBodyIndex :type Integer) (bFromSweep :type Boolean) (SweepResult :type Hit%20Result%20Structure%20%28by%20ref%29))
  (bind _asbp_third_person_character (Utilities|Casting|CastToBP_ThirdPersonCharacter (Game|Player|GetPlayerPawn 0)))
  (Default|EvCam _asbp_third_person_character)
  (Utilities|FlowControl|FlipFlop
    (:A
      (bind _newtrack_0 (Timeline|Timeline Play)
        (:Update
          (Transformation|SetRelativeLocation (Variables|Default|GetSm_game_ElevatorInside) (Math|Vector|MakeVector 0.0 0.0 (Math|Float|Lerp 0.0 (Variables|Default|GetB) _newtrack_0)) false false))))
    (:B
      (Timeline|Timeline Reverse))))

(fn ConstructionScript
  (Transformation|SetRelativeLocation (Variables|Default|GetSm_game_ElevatorInside) (Math|Vector|MakeVector 0.0 0.0 (Variables|Default|GetNew%20Location%20Z)) false false))