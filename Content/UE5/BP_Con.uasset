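; BP_Con is an actor that animates a cube and a text label from a single Timeline started on BeginPlay.
; The Timeline slides the cube along relative X, drives its "BsColor" material parameter and updates the text color.
; An event track uses a FlipFlop to toggle the label's visibility, making it blink.
; The construction script is empty, with an unconnected loop for spawning a row of static meshes left unused.
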(event EventBeginPlay
  (Rendering|Components|TextRender|SetText (Variables|Default|GetTextRender) (Variables|Default|GetValue))
  (Utilities|FlowControl|Sequence
    (:then_0
      (bind (_direction _newtrack_0 _newtrack_3) (Timeline|Timeline Play)
        (:Update
          (Transformation|SetRelativeLocation (Variables|Default|GetCube) (Math|Vector|MakeVector (* _newtrack_0 1e+02) 0.0 0.0) false false)
          (Rendering|Components|TextRender|SetTextRenderColor (Variables|Default|GetTextRender) (Variables|Default|GetValue_0))
          (Rendering|Material|SetVectorParameterValueonMaterials (Variables|Default|GetCube) "BsColor" (Math|Conversions|ToVector(LinearColor) _newtrack_3)))
        (:NewTrack_1
          (bind _isa (Utilities|FlowControl|FlipFlop)
            (:A
              _)
            (:B
              _))
          (Rendering|SetVisibility (Variables|Default|GetTextRender) _isa false))))
    (:then_1
      (Timeline|Timeline SetNewTime))))

(fn ConstructionScript)