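; BP_Door is an automatic sliding door that opens when something overlaps its Box trigger and closes when the overlap ends.
; A Timeline plays on begin overlap and reverses on end overlap, so the door animates both ways from one track.
; Its alpha lerps the relative locations of four door panels, sliding two apart vertically and two apart horizontally along X.
; Overlaps are not filtered by actor.
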(event OnComponentBeginOverlap(Box)
  (params (OverlappedComponent :type Primitive%20Component%20Object%20Reference) (OtherActor :type Actor%20Object%20Reference) (OtherComp :type Primitive%20Component%20Object%20Reference) (OtherBodyIndex :type Integer) (bFromSweep :type Boolean) (SweepResult :type Hit%20Result%20Structure%20%28by%20ref%29))
  (bind _newtrack_0 (Timeline|Timeline Play)
    (:Update
      (Transformation|SetRelativeLocation (Variables|Default|GetSm_door_Plane_003) (Math|Vector|MakeVector 0.0 0.0 (Math|Float|Lerp 0.0 1.5e+02 _newtrack_0)) false false)
      (Transformation|SetRelativeLocation (Variables|Default|GetSm_door_Plane) (Math|Vector|MakeVector 0.0 0.0 (Math|Float|Lerp 0.0 -1.5e+02 _newtrack_0)) false false)
      (Transformation|SetRelativeLocation (Variables|Default|GetSm_door_Plane_002) (Math|Vector|MakeVector (Math|Float|Lerp 0.0 1.2e+02 _newtrack_0) 0.0 0.0) false false)
      (Transformation|SetRelativeLocation (Variables|Default|GetSm_door_Plane_001) (Math|Vector|MakeVector (Math|Float|Lerp 0.0 -1.2e+02 _newtrack_0) 0.0 0.0) false false))))

(event OnComponentEndOverlap(Box)
  (params (OverlappedComponent :type Primitive%20Component%20Object%20Reference) (OtherActor :type Actor%20Object%20Reference) (OtherComp :type Primitive%20Component%20Object%20Reference) (OtherBodyIndex :type Integer))
  (bind _newtrack_0 (Timeline|Timeline Reverse)
    (:Update
      (Transformation|SetRelativeLocation (Variables|Default|GetSm_door_Plane_003) (Math|Vector|MakeVector 0.0 0.0 (Math|Float|Lerp 0.0 1.5e+02 _newtrack_0)) false false)
      (Transformation|SetRelativeLocation (Variables|Default|GetSm_door_Plane) (Math|Vector|MakeVector 0.0 0.0 (Math|Float|Lerp 0.0 -1.5e+02 _newtrack_0)) false false)
      (Transformation|SetRelativeLocation (Variables|Default|GetSm_door_Plane_002) (Math|Vector|MakeVector (Math|Float|Lerp 0.0 1.2e+02 _newtrack_0) 0.0 0.0) false false)
      (Transformation|SetRelativeLocation (Variables|Default|GetSm_door_Plane_001) (Math|Vector|MakeVector (Math|Float|Lerp 0.0 -1.2e+02 _newtrack_0) 0.0 0.0) false false))))

(fn ConstructionScript)