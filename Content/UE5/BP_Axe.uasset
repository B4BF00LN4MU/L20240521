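; BP_Axe is a swinging axe obstacle that reacts when the third-person character touches it.
; On BeginPlay a timeline starts from a random time, so placed axes can swing out of sync, and its track lerps the mesh pitch between negative and positive RotVal.
; A Box overlap casts the other actor to BP_ThirdPersonCharacter and calls its EvSim event.
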(event OnComponentBeginOverlap(Box)
  (params (OverlappedComponent :type Primitive%20Component%20Object%20Reference) (OtherActor :type Actor%20Object%20Reference) (OtherComp :type Primitive%20Component%20Object%20Reference) (OtherBodyIndex :type Integer) (bFromSweep :type Boolean) (SweepResult :type Hit%20Result%20Structure%20%28by%20ref%29))
  (bind _asbp_third_person_character (Utilities|Casting|CastToBP_ThirdPersonCharacter OtherActor))
  (Default|EvSim _asbp_third_person_character))

(event EventBeginPlay
  (bind _rotval (Variables|Default|GetrotVal))
  ;[1 1 1] 회전 애니메이션
  (Utilities|FlowControl|Sequence
    (:then_0
      (bind _newtrack_0 (Timeline|Timeline SetNewTime)
        (:Update
          (Transformation|SetRelativeRotation (Variables|Default|GetSm_game_ax) (Math|Rotator|MakeRotator 0.0 (Math|Float|Lerp (* _rotval -1.0) _rotval _newtrack_0) 0.0) false false))))
    (:then_1
      (Timeline|Timeline Play))))

(fn ConstructionScript)